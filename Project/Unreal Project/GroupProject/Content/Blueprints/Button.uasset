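; Interactive button actor that toggles an emergency light flag and plays a press animation.
; Each ButtonPress event flips EmergencyLightOn, even if the animation is still running.
; A timeline drives the Button component's relative location, with IsPressed blocking a restart until it finishes.
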(event Custom|Button%20Press
  (Utilities|FlowControl|Sequence
    (:then_0
      (if (Variables|Default|GetemergencyLightOn)
        (Variables|Default|SetemergencyLightOn false)
        (else
          (Variables|Default|SetemergencyLightOn true))))
    (:then_1
      (if (not (Variables|Default|GetisPressed))
        (Variables|Default|SetisPressed true)
        (bind _newtrack_0 (Timeline|Timeline_0 PlayFromStart)
          (:Update
            (Transformation|SetRelativeLocation (Variables|Default|GetButton) _newtrack_0 false false))
          (:Finished
            (Variables|Default|SetisPressed false)))))))

(fn ConstructionScript)