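; Corridor actor that dresses itself with a pipe system and an overhead emergency light when play begins.
; It spawns PipeSystem3 and TopEmergancyLight2 at hard-coded offsets from the static mesh's world location.
; The locator transform comes from location alone, so offsets and spawned actors ignore the corridor's rotation and scale.
; The light takes its scale from the EmergancyLightScale variable, and the construction script is empty.
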(event EventBeginPlay
  ;[1 1 1] Static Mesh Locator
  (Variables|Default|SetStatic%20Mesh%20Locator (Math|Conversions|ToTransform(Vector) (Transformation|GetWorldLocation (Variables|Default|GetStaticMesh))))
  (Game|SpawnActorfromClass "/Game/Blueprints/PipeSystem3.PipeSystem3_C" (Math|Transform|MakeTransform (Math|Transform|TransformLocation (Variables|Default|GetStatic%20Mesh%20Locator) "-46.000000,6.000000,-130.000000")) "Undefined" 0 0)
  (Game|SpawnActorfromClass "/Game/Blueprints/topEmergancyLight2.topEmergancyLight2_C" (Math|Transform|MakeTransform (Math|Transform|TransformLocation (Variables|Default|GetStatic%20Mesh%20Locator) "-60.000000,0.000000,445.000000") "0,0.000000, 0" (Variables|Default|GetEmergancy%20Light%20Scale)) "Undefined" 0 0))

(event Collision|EventActorBeginOverlap
  (params (OtherActor :type Actor%20Object%20Reference)))

(event EventTick
  (params (DeltaSeconds :type Float%20%28single-precision%29)))

(fn ConstructionScript)