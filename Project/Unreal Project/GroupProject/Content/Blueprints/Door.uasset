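; Sliding double door Blueprint that either opens or signals that it is locked when OpenDoor is called.
; When unlocked, a timeline slides both panels as a sound plays and the lock light turns green, with a flag blocking re-triggers.
; When locked, a second timeline lerps the light's color through a dynamic material instance created on each update.
; The Action input calls RaycastInput on the player's ThirdPersonCharacter.
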(event Custom|OpenDoor
  (bind _lock_light (Variables|Default|GetLock_Light))
  (if (Variables|Default|GetisLocked)
    ;[1 1 1] Locked Door
    (if (not (Variables|Default|GetlockLightPlaying))
      (Utilities|FlowControl|Sequence
        (:then_0
          (Development|PrintString "Door Locked" true true "(R=0.870000,G=0.000000,B=0.000000,A=1.000000)"))
        (:then_1
          (Variables|Default|SetlockLightPlaying true)
          (bind _newtrack_1 (Timeline|Timeline_2 PlayFromStart)
            (:Update
              (bind _returnvalue (Rendering|Material|CreateDynamicMaterialInstance _lock_light 0 "/Game/Materials/ERed.ERed" "None" :!class /Script/Engine.PrimitiveComponent))
              (Rendering|Material|SetScalarParameterValueonMaterials _lock_light "Emission" 1e+02)
              (Rendering|Material|SetVectorParameterValue _returnvalue "Color" (Math|Color|Lerp(LinearColor) "(R=0.275849,G=0.492738,B=0.729167,A=1.000000)" "(R=0.870000,G=0.000000,B=0.000000,A=1.000000)" _newtrack_1) :!class /Script/Engine.MaterialInstanceDynamic))
            (:Finished
              (Variables|Default|SetlockLightPlaying false))))))
    (else
      ;[1 1 1] Open Door
      (if (not (Variables|Default|GetisOpening))
        (Audio|Components|Audio|Play (Variables|Default|GetDoor_Sound) 0.9)
        (Rendering|Material|SetMaterial (Variables|Default|GetLock_Light) 0 "/Game/Materials/EGreen.EGreen")
        (Variables|Default|SetisOpening true)
        (bind (_direction _right_movement _left_movement) (Timeline|Timeline_0 PlayFromStart)
          (:Update
            (Utilities|FlowControl|Sequence
              (:then_0
                (Transformation|SetRelativeLocation (Variables|Default|GetDoor_Right) _right_movement false false))
              (:then_1
                (Transformation|SetRelativeLocation (Variables|Default|GetDoor_Left) _left_movement false false))))
          (:Finished
            (Variables|Default|SetisOpening false)
            (Rendering|Material|SetMaterial (Variables|Default|GetLock_Light) 0 0)))))))

(event Input|ActionEvents|InputActionAction
  (params (Key :type Key%20Structure))
  ;[1 1 1] Open Door
  ;;[1 1 1] Raycast Input
  (:Pressed
    (bind _asthird_person_character (Utilities|Casting|CastToThirdPersonCharacter (Game|GetPlayerCharacter 0)))
    (Default|RaycastInput _asthird_person_character)))

(fn ConstructionScript)