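; Sliding door actor that moves its Door component along relative Z when OpenDoor is called while something is in range.
; Actor begin and end overlap events toggle WithinOpeningRange without filtering which actor triggered them.
; DoorSetting selects the FullyOpen, HalfOpen or Broken timeline to drive the movement, always playing from start.
; IsOpening tracks playback but never blocks retriggering, and the graph has no closing logic.
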(event Custom|OpenDoor
  (bind _door (Variables|Default|GetDoor))
  (bind _xcord (Variables|Default|GetxCord))
  (bind _ycord (Variables|Default|GetyCord))
  (Development|PrintString "Door")
  (if (Variables|Default|GetWithinOpeningRange)
    (Variables|Default|SetIsOpening true)
    (switch int (Variables|Default|GetDoorSetting)
      (:0
        ;[1 1 1] Comment
        (bind _newtrack_0 (Timeline|FullyOpen PlayFromStart)
          (:Update
            (Transformation|SetRelativeLocation (Variables|Default|GetDoor) (Math|Vector|MakeVector _xcord _ycord _newtrack_0) false false))
          (:Finished
            ;[1 1 1] Comment
            (Variables|Default|SetIsOpening false :!label _label))))
      (:1
        ;[1 1 1] Comment
        (bind _newtrack_0_2 (Timeline|HalfOpen PlayFromStart)
          (:Update
            (Transformation|SetRelativeLocation _door (Math|Vector|MakeVector _xcord _ycord _newtrack_0_2) false false))
          (:Finished
            (goto _label))))
      (:2
        ;[1 1 1] Comment
        (bind _newtrack_0_3 (Timeline|broken PlayFromStart)
          (:Update
            (Transformation|SetRelativeLocation _door (Math|Vector|MakeVector _xcord _ycord _newtrack_0_3) false false))
          (:Finished
            (goto _label)))))
    (else
      (Development|PrintString "FALSE"))))

(event EventBeginPlay
  ;[1 1 1] Comment
)

(event EventTick
  (params (DeltaSeconds :type Float%20%28single-precision%29)))

(event Collision|EventActorBeginOverlap
  (params (OtherActor :type Actor%20Object%20Reference))
  ;[1 1 1] Comment
  (Variables|Default|SetWithinOpeningRange true)
  (Development|PrintString "within Opening Range"))

(event Collision|EventActorEndOverlap
  (params (OtherActor :type Actor%20Object%20Reference))
  ;[1 1 1] Comment
  (Variables|Default|SetWithinOpeningRange false)
  (Development|PrintString "Not Within Opening Range"))

(fn ConstructionScript)