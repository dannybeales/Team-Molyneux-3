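; Overhead emergency light actor with a rotating spotlight and flickering floor light, switching between red and white based on Button state.
; Tick spins SpotLight by LightRotationSpeed scaled by delta time and toggles FloorSpotLight visibility.
; A zero-delay loop from BeginPlay polls every Button's EmergencyLightOn, setting white when true and red when false, so the last Button wins.
; The construction script sets the initial spotlight color and creates a dynamic material.
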(event EventBeginPlay
  (bind _spotlight (Variables|Default|GetSpotLight))
  (bind _relativerotation (Variables|/Script/Engine.SceneComponent|GetRelativeRotation _spotlight))
  (bind (_roll _pitch _yaw) (Math|Rotator|BreakRotator _relativerotation))
  (Utilities|FlowControl|Sequence
    (:then_0
      ;[1 1 1] Red Light Rotation
      (Transformation|SetRelativeRotation _spotlight (Math|Rotator|MakeRotator _roll _pitch (+ _yaw (* (Variables|Default|GetLight%20Rotation%20Speed) (stale EventTick DeltaSeconds)))) false false)
      ;[1 1 1] Makes Lights Flicker
      (Rendering|ToggleVisibility (Variables|Default|GetFloorSpotLight) false))
    (:then_1
      (Utilities|FlowControl|Sequence :!label _label
        (:then_0
          (Utilities|FlowControl|Delay 0.0)
          (goto _label))
        (:then_1
          (bind _outactors (Actor|GetAllActorsOfClass "/Game/Blueprints/Button.Button_C"))
          (for _array_element _outactors
            (bind _output_get (Variables|Default|SetemergencyLight (Variables|/Game/Blueprints/Button.Button_C|GetemergencyLightOn _array_element)))
            (if _output_get
              (Rendering|Material|SetMaterial (Variables|Default|GetStaticMesh) 3 "/Game/Materials/TopLight.TopLight")
              (Rendering|Components|Light|SetLightColor (Variables|Default|GetFloorSpotLight) "(R=1.000000,G=1.000000,B=1.000000,A=1.000000)" true)
              (Rendering|Components|Light|SetLightColor (Variables|Default|GetPointLight) "(R=1.000000,G=1.000000,B=1.000000,A=1.000000)" true)
              (Rendering|Components|Light|SetLightColor (Variables|Default|GetSpotLight) "(R=1.000000,G=1.000000,B=1.000000,A=1.000000)" true)
              (else
                (Rendering|Material|SetMaterial (Variables|Default|GetStaticMesh) 3 "/Game/Meshes/M_Floor_Light_Inst1.M_Floor_Light_Inst1")
                (Rendering|Components|Light|SetLightColor (Variables|Default|GetFloorSpotLight) "(R=1.000000,G=0.333333,B=0.333333,A=1.000000)" true)
                (Rendering|Components|Light|SetLightColor (Variables|Default|GetPointLight) "(R=1.000000,G=0.000000,B=0.000000,A=1.000000)" true)
                (Rendering|Components|Light|SetLightColor (Variables|Default|GetSpotLight) "(R=1.000000,G=0.000000,B=0.000000,A=1.000000)" true)))))))))

(event Collision|EventActorBeginOverlap
  (params (OtherActor :type Actor%20Object%20Reference)))

(event EventTick
  (params (DeltaSeconds :type Float%20%28single-precision%29))
  (bind _spotlight (Variables|Default|GetSpotLight))
  (bind _relativerotation (Variables|/Script/Engine.SceneComponent|GetRelativeRotation _spotlight))
  (bind (_roll _pitch _yaw) (Math|Rotator|BreakRotator _relativerotation))
  ;[1 1 1] Red Light Rotation
  (Transformation|SetRelativeRotation _spotlight (Math|Rotator|MakeRotator _roll _pitch (+ _yaw (* (Variables|Default|GetLight%20Rotation%20Speed) DeltaSeconds))) false false)
  ;[1 1 1] Makes Lights Flicker
  (Rendering|ToggleVisibility (Variables|Default|GetFloorSpotLight) false))

(fn ConstructionScript
  ;[1 1 1] Set Light Colors
  (Rendering|Components|Light|SetLightColor (Variables|Default|GetSpotLight) (Variables|Default|GetAlarm%20On%20Light%20Color) true)
  ;[1 1 1] Build the MID
  (bind _returnvalue (Rendering|Material|CreateDynamicMaterialInstance (Variables|Default|GetStaticMesh) 0 0 "None" :!class /Script/Engine.PrimitiveComponent))
  (Variables|Default|SetAlarm%20Material _returnvalue))