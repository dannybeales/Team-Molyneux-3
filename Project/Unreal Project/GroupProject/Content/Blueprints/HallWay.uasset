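; Hallway actor that switches its mesh and lights between normal and emergency lighting.
; Every Tick it scans all Button actors and, following each one's EmergencyLightOn flag, swaps two mesh materials and shows or hides four spotlights, so the last Button found decides the result.
; BeginPlay caches the mesh location as a transform for pipe system and emergency light spawning, but that spawn logic is disconnected and never runs.
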(event EventBeginPlay
  ;[1 1 1] Static Mesh Locator
  (Variables|Default|SetStatic%20Mesh%20Locator (Math|Conversions|ToTransform(Vector) (Transformation|GetWorldLocation (Variables|Default|GetStaticMesh)))))

(event EventTick
  (params (DeltaSeconds :type Float%20%28single-precision%29))
  (bind _staticmesh (Variables|Default|GetStaticMesh))
  (bind _spotlight (Variables|Default|GetSpotLight))
  ;[1 1 1] Emergency Light Toggle
  (bind _outactors (Actor|GetAllActorsOfClass "/Game/Blueprints/Button.Button_C"))
  (for _array_element _outactors
    (bind _output_get (Variables|Default|SetemergencyLight (Variables|/Game/Blueprints/Button.Button_C|GetemergencyLightOn _array_element)))
    (if _output_get
      (Rendering|Material|SetMaterial _staticmesh 7 "/Game/Materials/EBlue.EBlue")
      (Rendering|Material|SetMaterial _staticmesh 2 "/Game/Materials/TopLight.TopLight")
      (Rendering|SetVisibility _spotlight true false)
      (else
        (Rendering|Material|SetMaterial _staticmesh 7 "/Game/Meshes/HallWay/FloorLights.FloorLights")
        (Rendering|Material|SetMaterial _staticmesh 2 "/Game/Meshes/HallWay/Lights.Lights")
        (Rendering|SetVisibility _spotlight false false)))))

(fn ConstructionScript)